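; Paper2D runner character that constantly moves along +X, with its speed driven by alternating left and right power presses.
; Each alternating press raises MaxWalkSpeed up to a cap, while Tick steadily drains it, both scaled by curves sampled at current velocity.
; Tick also switches idle and run flipbooks, scales run playback rate with speed, and plays footsteps on specific frames through a resettable do-once.
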(event Input|EnhancedActionEvents|EnhancedInputActionIA_PowerLeft
  (params (ActionValue :type Boolean) (ElapsedSeconds :type Float%20%28double-precision%29) (TriggeredSeconds :type Float%20%28double-precision%29) (InputAction :type Input%20Action%20Object%20Reference :default "/Game/InputSection/Actions/IA_PowerLeft.IA_PowerLeft"))
  (:Started
    (if (Utilities|Enum|NotEqual(Enum) (Variables|Default|GetLastInput) "NewEnumerator1")
      (Variables|Default|SetLastInput "NewEnumerator1")
      (CallFunction|IncreaseSpeed))))

(event Input|EnhancedActionEvents|EnhancedInputActionIA_PowerRight
  (params (ActionValue :type Boolean) (ElapsedSeconds :type Float%20%28double-precision%29) (TriggeredSeconds :type Float%20%28double-precision%29) (InputAction :type Input%20Action%20Object%20Reference :default "/Game/InputSection/Actions/IA_PowerRight.IA_PowerRight"))
  (:Started
    (if (Utilities|Enum|NotEqual(Enum) (Variables|Default|GetLastInput) "NewEnumerator2")
      (Variables|Default|SetLastInput "NewEnumerator2")
      (CallFunction|IncreaseSpeed))))

(event EventBeginPlay
  (bind _asplayer_controller (Utilities|Casting|CastToPlayerController (Pawn|GetController)))
  (Input|AddMappingContext (PlayerController|LocalPlayerSubsystems|GetEnhancedInputLocalPlayerSubsystem _asplayer_controller) "/Game/InputSection/IMC_Runner.IMC_Runner" 0 "(bIgnoreAllPressedKeysUntilRelease=True,bForceImmediately=False)"))

(event Collision|EventActorBeginOverlap
  (params (OtherActor :type Actor%20Object%20Reference)))

(event EventTick
  (params (DeltaSeconds :type Float%20%28single-precision%29))
  (bind _sprite (Variables|Default|GetSprite))
  (bind _returnvalue (Class|PaperFlipbookComponent|GetPlaybackPositioninFrames _sprite))
  (Pawn|Input|AddMovementInput "1.000000,0.000000,0.000000" 1.0 false)
  (CallFunction|DecreaseSpeed DeltaSeconds)
  (CallFunction|UpdateFlipbook)
  (CallFunction|SpriteRunPlayRate)
  (if (== (Class|PaperFlipbookComponent|GetFlipbook (Variables|Default|GetSprite)) "/Game/Assets/Runner/PF_RunRunner.PF_RunRunner")
    (if (or (== _returnvalue 1) (== _returnvalue 5))
      (|DoOnceMultiInput :!label _label
        (:A%20Out
          (Audio|PlaySound2D "/Game/Sounds/Footsteps/S_StepsCue.S_StepsCue" 1.0 1.0 0.0 0 0)))
      (else
        (goto _label Reset%20In)))))

(fn ConstructionScript)

(fn IncreaseSpeed
  (Variables|/Script/Engine.CharacterMovementComponent|SetMaxWalkSpeed (Variables|Character|GetCharacterMovement) (Math|Float|Clamp(Float) (+ (Variables|/Script/Engine.CharacterMovementComponent|GetMaxWalkSpeed (Variables|Character|GetCharacterMovement)) (* (Math|Curves|GetFloatValue (Variables|Default|GetSpeedIncreaseRamp) (Math|Vector|VectorLength (Variables|/Script/Engine.MovementComponent|GetVelocity (Variables|Character|GetCharacterMovement)))) (Variables|Default|GetSpeedUpPerTouch))) 0.0 (Variables|Default|GetMaxSpeed))))

(fn DecreaseSpeed
  (params (FrameCounterDelta :type Float%20%28double-precision%29))
  (Variables|/Script/Engine.CharacterMovementComponent|SetMaxWalkSpeed (Variables|Character|GetCharacterMovement) (Math|Float|Max(Float) (- (Variables|/Script/Engine.CharacterMovementComponent|GetMaxWalkSpeed (Variables|Character|GetCharacterMovement)) (* FrameCounterDelta (* (Variables|Default|GetSpeedMultiplex) (Math|Curves|GetFloatValue (Variables|Default|GetSpeedDecreaseRamp) (Math|Vector|VectorLength (Variables|/Script/Engine.MovementComponent|GetVelocity (Variables|Character|GetCharacterMovement))))))) 0.0)))

(fn UpdateFlipbook
  (Sprite|SetFlipbook (Variables|Default|GetSprite) (select (> (Math|Vector|VectorLength (Variables|/Script/Engine.MovementComponent|GetVelocity (Variables|Character|GetCharacterMovement))) 0.0) "/Game/Assets/Runner/PF_RunRunner.PF_RunRunner" "/Game/Assets/Runner/PF_IdleRunner.PF_IdleRunner")))

(fn SpriteRunPlayRate
  (if (== (Class|PaperFlipbookComponent|GetFlipbook (Variables|Default|GetSprite)) "/Game/Assets/Runner/PF_RunRunner.PF_RunRunner")
    (Components|Timeline|SetPlayRate (Variables|Default|GetSprite) (/ (Math|Vector|VectorLength (Variables|/Script/Engine.MovementComponent|GetVelocity (Variables|Character|GetCharacterMovement))) (Variables|Default|GetMaxSpeed)))
    (else
      (Components|Timeline|SetPlayRate (Variables|Default|GetSprite) 1.0))))