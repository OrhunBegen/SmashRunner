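; BP_Field is a Paper2D stage field that builds itself from repeated sprite segments in the Construction Script.
; It places StageParts copies of the field sprite along X, spaced by StageLength.
; BoxExtend stretches the Stage1 and Stage2 boxes to span the whole row, and ColliderExtend re-centers them on it, keeping their Y and Z values.
; The event graph has no active logic.
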(event EventBeginPlay)

(event Collision|EventActorBeginOverlap
  (params (OtherActor :type Actor%20Object%20Reference)))

(event EventTick
  (params (DeltaSeconds :type Float%20%28single-precision%29)))

(fn ConstructionScript
  (bind _stage2 (Variables|Default|GetStage2))
  (bind _stage2_2 (Variables|Default|GetStage2))
  (for _index (range 0 (- (Variables|Default|GetStageParts) 1))
    (bind _returnvalue (AddComponent|AddPaperSpriteComponent false (Math|Transform|MakeTransform (Math|Vector|MakeVector (Math|Conversions|ToFloat(Integer) (* _index (Variables|Default|GetStageLength))) 0.0 0.0) "0, 0, 0" "1.000000,1.000000,1.000000")))
    (Rendering|Components|Sprite|SetSprite _returnvalue "/Game/Assets/Background/T_Field_Sprite.T_Field_Sprite"))
  (CallFunction|BoxExtend (Variables|Default|GetStage1) (Variables|Default|GetStage1))
  (CallFunction|BoxExtend _stage2 _stage2)
  (CallFunction|ColliderExtend (Variables|Default|GetStage1) (Variables|Default|GetStage1))
  (CallFunction|ColliderExtend _stage2_2 _stage2_2))

(fn BoxExtend
  (params (self2 :type Box%20Component%20Object%20Reference) (self3 :type Box%20Component%20Object%20Reference))
  (bind _returnvalue (Components|Box|GetScaledBoxExtent self3))
  (Components|Box|SetBoxExtent self2 (Math|Vector|MakeVector (Math|Conversions|ToFloat(Integer) (* (Variables|Default|GetStageParts) (/ (Variables|Default|GetStageLength) 2))) (.y _returnvalue) (.z _returnvalue)) true))

(fn ColliderExtend
  (params (self2 :type Scene%20Component%20Object%20Reference) (self3 :type Scene%20Component%20Object%20Reference))
  (bind _relativelocation (Variables|/Script/Engine.SceneComponent|GetRelativeLocation self3))
  (Transformation|SetRelativeLocation self2 (Math|Vector|MakeVector (Math|Conversions|ToFloat(Integer) (- (/ (* (Variables|Default|GetStageParts) (Variables|Default|GetStageLength)) 2) (/ (Variables|Default|GetStageLength) 2))) (.y _relativelocation) (.z _relativelocation)) false false))